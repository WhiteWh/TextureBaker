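; Texture baker Blueprint that bakes a palettized version of a source Texture using a Palette texture.
; It requires both textures to be valid, then registers a Texture2D output named after the source, matching its size and power-of-two padding, with configurable sRGB and compression.
; Baking feeds both prepared textures into a dynamic instance of ProcessingMaterial and draws it across the output canvas, leaving the palette mapping to that material.
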(fn `BakeTexture`
  (params (Info :type "TextureBakerOutputInfo Structure") (bIsPreviewRender :type Boolean) (Canvas :type "Canvas Object Reference"))
  (returns (ReturnValue :type Boolean))
  (bind _returnvalue (`self.PrepareTexture` (`self.Texture`) (make `TextureBakerResourceRequirements` true)))
  (bind _returnvalue_2 (`self.PrepareTexture` (`self.Palette`) (make `TextureBakerResourceRequirements` true)))
  (bind _returnvalue_3 (`self.PrepareDynamicMaterialInstance` (`self.ProcessingMaterial`)))
  (`MaterialInstanceDynamic.SetTextureParameterValue` _returnvalue_3 "Texture" _returnvalue)
  (`MaterialInstanceDynamic.SetTextureParameterValue` _returnvalue_3 "Palette" _returnvalue_2)
  (`Canvas.K2_DrawMaterial` Canvas _returnvalue_3 (0.0 0.0) (`KismetMathLibrary.Conv_IntPointToVector2D` Info_OutputDimensions) (0.0 0.0) (1.0 1.0) 0.0 (0.5 0.5))
  (return true))

(fn `InitialSettingsIsValid`
  (returns (ReturnValue :type Boolean))
  (return (and (`KismetSystemLibrary.IsValid` (`self.Texture`)) (`KismetSystemLibrary.IsValid` (`self.Palette`)))))

(fn `RegisterOutputTarget`
  (params (DirectoryPath :type String) (OutputTargets :type "TextureBakerOutputList Structure (by ref)"))
  (bind _texture (`self.Texture`))
  (`TextureBakerOutputBlueprintLibrary.AddTexture2DOutput` OutputTargets (make `TextureBakerOutputInfo` (make `IntPoint` (`Texture2D.Blueprint_GetSizeX` _texture) (`Texture2D.Blueprint_GetSizeY` _texture)) (`Texture.PowerOfTwoMode` _texture) (struct :`A` 1.0) "TMGS_FromTextureGroup" "TSF_BGRA8" "Saturate" "TF_Default" "TA_Wrap" "TA_Wrap" (`self.UseSRGB`) (`self.CompressionSettings`) (`self.CompressWithoutAlpha`)) (`KismetStringLibrary.JoinStringArray` (`|MakeArray` DirectoryPath (`KismetSystemLibrary.GetObjectName` _texture)) "/") (`|CreateDelegate` :!event `BakeTexture`))
  (return))