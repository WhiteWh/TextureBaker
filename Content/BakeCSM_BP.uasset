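; Texture baker Blueprint that bakes a CSM texture from a required heightmap and an optional normal map.
; It registers one linear output at heightmap resolution, named from the heightmap's name with trimmed words, custom prefix and suffix, and "_DT".
; GenerateCSM prepares mipless inputs, picks the render material with or without normals, and draws it across the canvas, leaving the computation to that material.
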(fn `GenerateCSM`
  (params (Info :type "TextureBakerOutputInfo Structure") (bIsPreviewRender :type Boolean) (Canvas :type "Canvas Object Reference"))
  (returns (ReturnValue :type Boolean))
  (locals (LocalScreenSize :type "Vector2D Structure") (HeightmapEncoded :type "Texture2D Object Reference") (NormalmapEncoded :type "Texture2D Object Reference") (LocalRenderMaterial :type "MaterialInstanceDynamic Object Reference"))
  (`|ExecutionSequence`
    (:`then_0`
      (set `local.LocalScreenSize` (`KismetMathLibrary.Conv_IntPointToVector2D` Info_OutputDimensions))
      (bind _returnvalue (`self.PrepareTexture` (`self.Heightmap`) (make `TextureBakerResourceRequirements` true true "TMGS_NoMipmaps")))
      (set `local.HeightmapEncoded` _returnvalue))
    (:`then_1`
      (bind _normalmap (`self.NormalMap`)
        (:`then`
          (bind _returnvalue_2 (`self.PrepareTexture` _normalmap (make `TextureBakerResourceRequirements` true true "TMGS_NoMipmaps")))
          (set `local.NormalmapEncoded` _returnvalue_2)
          (bind _returnvalue_3 (`self.PrepareDynamicMaterialInstance` (`self.RenderMaterial_WithNormals`)))
          (bind _output_get (set `local.LocalRenderMaterial` _returnvalue_3))
          (`MaterialInstanceDynamic.SetTextureParameterValue` _output_get "NormalMap" (`local.NormalmapEncoded`)))
        (:`else`)))
    (:`then_2`
      (`local.LocalRenderMaterial`
        (:`then`
          _)
        (:`else`
          (bind _returnvalue_4 (`self.PrepareDynamicMaterialInstance` (`self.RenderMaterial_WithoutNormals`)))
          (set `local.LocalRenderMaterial` _returnvalue_4)))
      (`MaterialInstanceDynamic.SetTextureParameterValue` (`local.LocalRenderMaterial`) "HeightMap" (`local.HeightmapEncoded`))
      (`Canvas.K2_DrawMaterial` (`local.Canvas`) (`local.LocalRenderMaterial`) (0.0 0.0) (`local.LocalScreenSize`) (0.0 0.0) (1.0 1.0) 0.0 (0.5 0.5))
      (return true))))

(fn `InitialSettingsIsValid`
  (returns (ReturnValue :type Boolean))
  (return (`KismetSystemLibrary.IsValid` (`self.Heightmap`))))

(fn `NameConstructor`
  (params (`CutFromStart-End` :type "IntPoint Structure") (TextureName :type String) (CustomPrefix :type String) (CustomSuffix :type String))
  (returns (ResultName :type String))
  (locals (NewNameArray :type "Array of String") (LastIndex :type Integer) (PTK_Words :type "Array of Integer"))
  (bind _cutfromstart_end_x (break `IntPoint` (`local.CutFromStart-End`)))
  (bind (_cutfromstart_end_x_2 _cutfromstart_end_y) (break `IntPoint` (`local.CutFromStart-End`)))
  (bind _cutfromstart_end_x_3 (break `IntPoint` (`local.CutFromStart-End`)))
  (bind _customprefix (`local.CustomPrefix`))
  (bind _customsuffix (`local.CustomSuffix`))
  (bind (_cutfromstart_end_x_4 _cutfromstart_end_y_2) (break `IntPoint` (`local.CutFromStart-End`)))
  (bind _output_get (set `local.NewNameArray` (`KismetStringLibrary.ParseIntoArray` TextureName "_")))
  (set `local.LastIndex` (`KismetArrayLibrary.Array_Length` _output_get))
  (`|ExecutionSequence`
    (:`then_0`
      (if (<= (- (- (`local.LastIndex`) _cutfromstart_end_x_2) _cutfromstart_end_y) 0)
        ;[1 1 1] If user cut all name, we have clear name array (PlaceHolder Add at last step)
        (`KismetArrayLibrary.Array_Clear` (`local.NewNameArray`))
        (else
          ;[1 1 1] Calculate Inverse Pending to kill indexes array (for native protected order) and Del name parts from name array
          (`|ExecutionSequence`
            (:`then_0`
              (if (> _cutfromstart_end_y_2 0)
                (for _index (range _cutfromstart_end_y_2)
                  (`KismetArrayLibrary.Array_Add` (`local.PTK_Words`) (- (`local.LastIndex`) (+ _index 1))))))
            (:`then_1`
              (if (> _cutfromstart_end_x_3 0)
                (for _index_2 (range _cutfromstart_end_x_3)
                  (`KismetArrayLibrary.Array_Add` (`local.PTK_Words`) (- (- _cutfromstart_end_x 1) _index_2)))))
            (:`then_2`
              (for _array_element (`local.PTK_Words`)
                (`KismetArrayLibrary.Array_Remove` (`local.NewNameArray`) _array_element)))))))
    (:`then_1`
      ;[1 1 1] Create result name, with custom prefix and sufix
      (`|ExecutionSequence`
        (:`then_0`
          ;;[1 1 1] Add custom Sufix\prefix only if is not empty
          (if (> (`KismetStringLibrary.Len` _customprefix) 0)
            (`KismetArrayLibrary.Array_Insert` (`local.NewNameArray`) _customprefix)))
        (:`then_1`
          (if (> (`KismetStringLibrary.Len` _customsuffix) 0)
            (`KismetArrayLibrary.Array_Add` (`local.NewNameArray`) _customsuffix)))
        (:`then_2`
          (if (== (`KismetArrayLibrary.Array_Length` (`local.NewNameArray`)) 0)
            (`KismetArrayLibrary.Array_Add` (`local.NewNameArray`)))
          (return (`KismetStringLibrary.JoinStringArray` (`local.NewNameArray`) "_")))))))

(fn `RegisterOutputTarget`
  (params (DirectoryPath :type String) (OutputTargets :type "TextureBakerOutputList Structure (by ref)"))
  (bind _heightmap (`self.Heightmap`))
  (bind _resultname (`self.NameConstructor` (`self.Cut Start-End Words`) (`KismetSystemLibrary.GetObjectName` (`self.Heightmap`)) (`self.Prefix`) (`self.Suffix`)))
  (`TextureBakerOutputBlueprintLibrary.AddTexture2DOutput` (`local.OutputTargets`) (make `TextureBakerOutputInfo` (make `IntPoint` (`Texture2D.Blueprint_GetSizeX` _heightmap) (`Texture2D.Blueprint_GetSizeY` _heightmap)) "None" (struct :`A` 1.0) "TMGS_FromTextureGroup" "TSF_BGRA8" "Saturate" "TF_Default" "TA_Wrap" "TA_Wrap" false "TC_VectorDisplacementmap") (`KismetStringLibrary.Concat_StrStr` (`local.DirectoryPath`) "/" _resultname "_DT") (`|CreateDelegate` :!event `GenerateCSM`))
  (return))

(fn `RenderCommonTargets`
  (params (bIsPreviewRender :type Boolean))
  (returns (ReturnValue :type Boolean))
  (locals (DMI :type "MaterialInstanceDynamic Object Reference"))
  (return false))