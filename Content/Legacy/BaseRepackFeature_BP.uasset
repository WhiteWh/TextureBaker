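; Editor-only base Blueprint for texture repack features, baking source textures through a material into a new saved texture asset.
; RunBake takes textures and material from empty override hooks, sizes render targets by the per-axis minimum resolution, and builds the output name from the first texture's name.
; Bake draws the material, optionally ping-ponging between two targets for iterative passes, before RT01 is saved.
; Source texture settings save and restore logic is disconnected.
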(fn `Bake`
  (params (CPUCycle :type Boolean) (CycleSteps :type Integer))
  (bind _rt01 (`self.RT01`))
  (bind _rt02 (`self.RT02`))
  (bind _returnvalue (`EditorLevelLibrary.GetEditorWorld`))
  (`KismetRenderingLibrary.DrawMaterialToRenderTarget` _returnvalue (`self.RT01`) (`self.DMI`))
  (if (`self.CPU_Cycle`)
    (for _index (range (+ (* (`local.CycleSteps`) 2) 1))
      (bind _returnvalue_2 (== (mod _index 2) 0))
      (`MaterialInstanceDynamic.SetTextureParameterValue` (`self.DMI`) "ID" (select `bool` _returnvalue_2 :`false` _rt02 :`true` _rt01))
      (`KismetRenderingLibrary.DrawMaterialToRenderTarget` _returnvalue (select `bool` _returnvalue_2 :`false` _rt01 :`true` _rt02) (`self.DMI`))))
  (return))

(fn `CreateDMI`
  (returns (DMI :type "MaterialInstanceDynamic Object Reference"))
  (return null))

(fn `CreateRT`
  (params (SRGB :type Boolean) (SecondRT :type Boolean))
  (bind _returnvalue (select `bool` SRGB :`false` "RTF_RGBA8" :`true` "RTF_RGBA8_SRGB" :!type "ETextureRenderTargetFormat Enum"))
  (bind (_outputtextureresolution_x _outputtextureresolution_y) (break `IntPoint` (`self.OutputTextureResolution`)))
  (bind (_outputtextureresolution_x_2 _outputtextureresolution_y_2) (break `IntPoint` (`self.OutputTextureResolution`)))
  (bind _returnvalue_2 (`EditorLevelLibrary.GetEditorWorld`))
  (bind _returnvalue_3 (`KismetRenderingLibrary.CreateRenderTarget2D` _returnvalue_2 _outputtextureresolution_x_2 _outputtextureresolution_y_2 _returnvalue))
  (bind _output_get (set `self.RT01` _returnvalue_3))
  (set `Texture.Filter` "TF_Nearest" _output_get)
  (if SecondRT
    (bind _returnvalue_4 (`KismetRenderingLibrary.CreateRenderTarget2D` _returnvalue_2 _outputtextureresolution_x _outputtextureresolution_y _returnvalue))
    (bind _output_get_2 (set `self.RT02` _returnvalue_4))
    (set `Texture.Filter` "TF_Nearest" _output_get_2)))

(fn `GetMaxTextureResolution`
  (bind (_outputtextureresolution_x _outputtextureresolution_y) (break `IntPoint` (`self.OutputTextureResolution`)))
  (for _array_element (`self.TextureArray`)
    (set `self.OutputTextureResolution` (make `IntPoint` (`KismetMathLibrary.Min` _outputtextureresolution_x (`Texture2D.Blueprint_GetSizeX` _array_element)) (`KismetMathLibrary.Min` _outputtextureresolution_y (`Texture2D.Blueprint_GetSizeY` _array_element))))))

(fn `NameConstructor`
  (params (`CutFromStart-End` :type "IntPoint Structure") (TextureName :type String) (CustomPrefix :type String) (CustomSuffix :type String) (TechSuffix :type String))
  (returns (ResultName :type String))
  (locals (LastIndex :type Integer) (PTK_Words :type "Array of Integer") (NewNameArray :type "Array of String"))
  (bind _cutfromstart_end_x (break `IntPoint` (`local.CutFromStart-End`)))
  (bind (_cutfromstart_end_x_2 _cutfromstart_end_y) (break `IntPoint` (`local.CutFromStart-End`)))
  (bind _cutfromstart_end_x_3 (break `IntPoint` (`local.CutFromStart-End`)))
  (bind _customprefix (`local.CustomPrefix`))
  (bind _customsuffix (`local.CustomSuffix`))
  (bind (_cutfromstart_end_x_4 _cutfromstart_end_y_2) (break `IntPoint` (`local.CutFromStart-End`)))
  (bind _newnamearray (`local.NewNameArray`))
  (bind _output_get (set `local.NewNameArray` (`KismetStringLibrary.ParseIntoArray` TextureName "_")))
  (set `local.LastIndex` (`KismetArrayLibrary.Array_Length` _output_get))
  (`|ExecutionSequence`
    (:`then_0`
      (if (<= (- (- (`local.LastIndex`) _cutfromstart_end_x_2) _cutfromstart_end_y) 0)
        ;[1 1 1] If user cut all name, we have clear name array (PlaceHolder Add at last step)
        (`KismetArrayLibrary.Array_Clear` (`local.NewNameArray`))
        (else
          ;[1 1 1] Calculate Inverse Pending to kill indexes array (for native protected order) and Del name parts from name array
          (`|ExecutionSequence`
            (:`then_0`
              (if (> _cutfromstart_end_y_2 0)
                (for _index (range _cutfromstart_end_y_2)
                  (`KismetArrayLibrary.Array_Add` (`local.PTK_Words`) (- (`local.LastIndex`) (+ _index 1))))))
            (:`then_1`
              (if (> _cutfromstart_end_x_3 0)
                (for _index_2 (range _cutfromstart_end_x_3)
                  (`KismetArrayLibrary.Array_Add` (`local.PTK_Words`) (- (- _cutfromstart_end_x 1) _index_2)))))
            (:`then_2`
              (for _array_element (`local.PTK_Words`)
                (`KismetArrayLibrary.Array_Remove` (`local.NewNameArray`) _array_element)))))))
    (:`then_1`
      ;[1 1 1] Create result name, with custom prefix and sufix
      (`|ExecutionSequence`
        (:`then_0`
          ;;[1 1 1] Add custom Sufix\prefix only if is not empty
          (if (> (`KismetStringLibrary.Len` _customprefix) 0)
            (`KismetArrayLibrary.Array_Insert` (`local.NewNameArray`) _customprefix)))
        (:`then_1`
          (if (> (`KismetStringLibrary.Len` _customsuffix) 0)
            (`KismetArrayLibrary.Array_Add` (`local.NewNameArray`) _customsuffix)))
        (:`then_2`
          (if (== (`KismetArrayLibrary.Array_Length` (`local.NewNameArray`)) 0)
            (`KismetArrayLibrary.Array_Add` _newnamearray))
          (`KismetArrayLibrary.Array_Add` _newnamearray (`local.TechSuffix`))
          (bind _output_get_2 (set `self.ResultName` (`KismetStringLibrary.Concat_StrStr` (`BlueprintPathsLibrary.MakePathRelativeTo` (`.Path` (break `DirectoryPath` (`self.Path`))) (`KismetSystemLibrary.GetProjectContentDirectory`)) "/" (`KismetStringLibrary.JoinStringArray` (`local.NewNameArray`) "_"))))
          (return _output_get_2))))))

(fn `RestoreTextureSettings`
  (return))

(fn `RunBake`
  (bind _texturearray (`self.SetTextureArray`))
  (set `self.TextureArray` _texturearray)
  (`self.SaveTextureSettings`)
  (`self.GetMaxTextureResolution`)
  (`self.NameConstructor` (`self.Cut Start-End Words`) (`KismetSystemLibrary.GetObjectName` (`|GetArrayItem` (`self.TextureArray`))) (`self.Prefix`) (`self.Suffix`) (`self.TechSuffix`))
  (`self.CreateRT` (`self.Color`) (`self.CPU_Cycle`))
  (bind _dmi (`self.CreateDMI`))
  (set `self.DMI` _dmi)
  (`self.Bake` (`self.CPU_Cycle`) (`self.CycleSteps`))
  (`self.SaveResultTexture`)
  (`self.RestoreTextureSettings`))

(fn `SaveResultTexture`
  (bind _returnvalue (`KismetRenderingLibrary.RenderTargetCreateStaticTexture2DEditorOnly` (`self.RT01`) (`self.ResultName`) (`self.ResultTextureCompression`) (`self.ResultTextureMipMaps`)))
  (set `Texture.LODGroup` (`self.ResultTextureLODGroup`) _returnvalue)
  (set `Texture.Filter` (`self.ResultTextureFilter`) _returnvalue)
  (set `Texture.CompressionNoAlpha` (`self.ResultTextureNoAlpha`) _returnvalue)
  (set `Texture.SRGB` (`self.ResultTexture_sRGB`) _returnvalue)
  (`EditorAssetLibrary.SaveLoadedAsset` _returnvalue false))

(fn `SaveTextureSettings`
  (return))

(fn `SetTextureArray`
  (returns (TextureArray :type "Array of Texture2D Object Reference"))
  (return))