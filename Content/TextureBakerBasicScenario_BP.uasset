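; Texture Baker scenario that bakes a source Texture into two same-sized BGRA8 assets suffixed _DT and _NM.
; RegisterOutputTarget builds paths through NameConstructor, which trims underscore-separated words from either end and adds optional prefix and suffix.
; DiffuseMap and NormalMap each draw the texture through a dynamic material, both currently using RenderMaterialNM.
; RenderCommonTargets runs a single-pass swap render target draw, then resolves, downsamples and releases it.
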(fn `DiffuseMap`
  (params (Info :type "TextureBakerOutputInfo Structure") (bIsPreviewRender :type Boolean) (Canvas :type "Canvas Object Reference"))
  (returns (ReturnValue :type Boolean))
  (bind _info_outputdimensions (break `TextureBakerOutputInfo` (`local.Info`)))
  (bind _returnvalue (`self.PrepareTexture` (`self.Texture`)))
  (bind _returnvalue_2 (`self.PrepareDynamicMaterialInstance` (`self.RenderMaterial_NM`)))
  (`MaterialInstanceDynamic.SetTextureParameterValue` _returnvalue_2 "Texture" _returnvalue)
  (`Canvas.K2_DrawMaterial` (`local.Canvas`) _returnvalue_2 (0.0 0.0) (`KismetMathLibrary.Conv_IntPointToVector2D` _info_outputdimensions) (0.0 0.0) (1.0 1.0) 0.0 (0.5 0.5))
  (return true))

(fn `InitialSettingsIsValid`
  (returns (ReturnValue :type Boolean))
  (return (`KismetSystemLibrary.IsValid` (`self.Texture`))))

(fn `NameConstructor`
  (params (`CutFromStart-End` :type "IntPoint Structure") (TextureName :type String) (CustomPrefix :type String) (CustomSuffix :type String))
  (returns (ResultName :type String))
  (locals (NewNameArray :type "Array of String") (LastIndex :type Integer) (PTK_Words :type "Array of Integer"))
  (bind _cutfromstart_end_x (break `IntPoint` (`local.CutFromStart-End`)))
  (bind (_cutfromstart_end_x_2 _cutfromstart_end_y) (break `IntPoint` (`local.CutFromStart-End`)))
  (bind _cutfromstart_end_x_3 (break `IntPoint` (`local.CutFromStart-End`)))
  (bind _customprefix (`local.CustomPrefix`))
  (bind _customsuffix (`local.CustomSuffix`))
  (bind (_cutfromstart_end_x_4 _cutfromstart_end_y_2) (break `IntPoint` (`local.CutFromStart-End`)))
  (bind _output_get (set `local.NewNameArray` (`KismetStringLibrary.ParseIntoArray` TextureName "_")))
  (set `local.LastIndex` (`KismetArrayLibrary.Array_Length` _output_get))
  (`|ExecutionSequence`
    (:`then_0`
      (if (<= (- (- (`local.LastIndex`) _cutfromstart_end_x_2) _cutfromstart_end_y) 0)
        ;[1 1 1] If user cut all name, we have clear name array (PlaceHolder Add at last step)
        (`KismetArrayLibrary.Array_Clear` (`local.NewNameArray`))
        (else
          ;[1 1 1] Calculate Inverse Pending to kill indexes array (for native protected order) and Del name parts from name array
          (`|ExecutionSequence`
            (:`then_0`
              (if (> _cutfromstart_end_y_2 0)
                (for _index (range _cutfromstart_end_y_2)
                  (`KismetArrayLibrary.Array_Add` (`local.PTK_Words`) (- (`local.LastIndex`) (+ _index 1))))))
            (:`then_1`
              (if (> _cutfromstart_end_x_3 0)
                (for _index_2 (range _cutfromstart_end_x_3)
                  (`KismetArrayLibrary.Array_Add` (`local.PTK_Words`) (- (- _cutfromstart_end_x 1) _index_2)))))
            (:`then_2`
              (for _array_element (`local.PTK_Words`)
                (`KismetArrayLibrary.Array_Remove` (`local.NewNameArray`) _array_element)))))))
    (:`then_1`
      ;[1 1 1] Create result name, with custom prefix and sufix
      (`|ExecutionSequence`
        (:`then_0`
          ;;[1 1 1] Add custom Sufix\prefix only if is not empty
          (if (> (`KismetStringLibrary.Len` _customprefix) 0)
            (`KismetArrayLibrary.Array_Insert` (`local.NewNameArray`) _customprefix)))
        (:`then_1`
          (if (> (`KismetStringLibrary.Len` _customsuffix) 0)
            (`KismetArrayLibrary.Array_Add` (`local.NewNameArray`) _customsuffix)))
        (:`then_2`
          (if (== (`KismetArrayLibrary.Array_Length` (`local.NewNameArray`)) 0)
            (`KismetArrayLibrary.Array_Add` (`local.NewNameArray`)))
          (return (`KismetStringLibrary.JoinStringArray` (`local.NewNameArray`) "_")))))))

(fn `NormalMap`
  (params (Info :type "TextureBakerOutputInfo Structure") (bIsPreviewRender :type Boolean) (Canvas :type "Canvas Object Reference"))
  (returns (ReturnValue :type Boolean))
  (bind _info_outputdimensions (break `TextureBakerOutputInfo` (`local.Info`)))
  (bind _returnvalue (`self.PrepareTexture` (`self.Texture`)))
  (bind _returnvalue_2 (`self.PrepareDynamicMaterialInstance` (`self.RenderMaterial_NM`)))
  (`MaterialInstanceDynamic.SetTextureParameterValue` _returnvalue_2 "Texture" _returnvalue)
  (`Canvas.K2_DrawMaterial` (`local.Canvas`) _returnvalue_2 (0.0 0.0) (`KismetMathLibrary.Conv_IntPointToVector2D` _info_outputdimensions) (0.0 0.0) (1.0 1.0) 0.0 (0.5 0.5))
  (return true))

(fn `RegisterOutputTarget`
  (params (DirectoryPath :type String))
  (returns (OutputTargets :type "Array of TextureBakerOutputWriteout Structure"))
  (bind _directorypath (`local.DirectoryPath`))
  (bind _texture (`self.Texture`))
  (bind _texturebakeroutputinfo (make `TextureBakerOutputInfo` (make `IntPoint` (`Texture2D.Blueprint_GetSizeX` _texture) (`Texture2D.Blueprint_GetSizeY` _texture)) false "TSF_BGRA8"))
  (bind _resultname (`self.NameConstructor` (`self.Cut Start-End Words`) (`KismetSystemLibrary.GetObjectName` (`self.Texture`)) (`self.Prefix`) (`self.Suffix`)))
  (return (`|MakeArray` (`TextureBakerOutputBlueprintLibrary.MakeOutputWriteout` (`KismetStringLibrary.Concat_StrStr` _directorypath "/" _resultname "_DT") _texturebakeroutputinfo (`|CreateDelegate` :!event `DiffuseMap`)) (`TextureBakerOutputBlueprintLibrary.MakeOutputWriteout` (`KismetStringLibrary.Concat_StrStr` _directorypath "/" _resultname "_NM") _texturebakeroutputinfo (`|CreateDelegate` :!event `NormalMap`)))))

(fn `RenderCommonTargets`
  (params (bIsPreviewRender :type Boolean))
  (returns (ReturnValue :type Boolean))
  (locals (DMI :type "MaterialInstanceDynamic Object Reference"))
  (bind _returnvalue (`self.PrepareDynamicMaterialInstance` null))
  (set `local.DMI` _returnvalue)
  (bind _returnvalue_2 (`self.CreateTemporarySwapRT` 5 (make `IntPoint` 1024 1024) "RTF_RGBA8"))
  (for _ (range 1)
    (bind (_history _screensize _returnvalue_3) (`TextureBakerOutputBlueprintLibrary.DrawToSwapRT` _returnvalue_2))
    (`MaterialInstanceDynamic.SetTextureParameterValue` (`local.DMI`) "Texture" (`|GetArrayItem` _history))
    (`Canvas.K2_DrawMaterial` _returnvalue_3 (`local.DMI`) (0.0 0.0) (`KismetMathLibrary.Conv_IntPointToVector2D` _screensize) (0.0 0.0) (1.0 1.0) 0.0 (0.5 0.5)))
  (bind _returnvalue_4 (`TextureBakerOutputBlueprintLibrary.ResolveTemporarySwapRT` _returnvalue_2))
  (bind _returnvalue_5 (`self.DownsampleTexture` _returnvalue_4 0 "TMGS_SimpleAverage"))
  (bind _returnvalue_6 (`self.ReleaseTemporaryResource` _returnvalue_5))
  (return _returnvalue_6))