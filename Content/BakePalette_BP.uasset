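; Texture baker Blueprint that turns an array of palette colors into a small lookup texture asset, one color per pixel.
; It validates the name and palette, then registers an output sized as either a square or a tighter near-square rectangle, with BakePalette as its render callback.
; The callback draws colors row by row, leaving spare pixels as the first color.
; Nearest filtering, clamping and no mipmaps keep entries distinct.
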(fn `BakePalette`
  (params (Info :type "TextureBakerOutputInfo Structure") (bIsPreviewRender :type Boolean) (Canvas :type "Canvas Object Reference"))
  (returns (ReturnValue :type Boolean))
  (for _index (range (`KismetArrayLibrary.Array_Length` (`self.Palette`)))
    (`Canvas.K2_DrawBox` (`local.Canvas`) (+ (`KismetMathLibrary.MakeVector2D` (`KismetMathLibrary.Conv_IntToDouble` (mod _index (break `IntPoint` (break `TextureBakerOutputInfo` Info)))) (`KismetMathLibrary.Conv_IntToDouble` (/ _index (break `IntPoint` (break `TextureBakerOutputInfo` Info))))) 0.5) (0.5 0.5) 1.0 (`|GetArrayItem` (`self.Palette`) _index)))
  (return true))

(fn `InitialSettingsIsValid`
  (returns (ReturnValue :type Boolean))
  (return (and (not (`KismetStringLibrary.IsEmpty` (`self.TextureName`))) (> (`KismetArrayLibrary.Array_Length` (`self.Palette`)) 0))))

(fn `RegisterOutputTarget`
  (params (DirectoryPath :type String) (OutputTargets :type "TextureBakerOutputList Structure (by ref)"))
  (bind _palette (`self.Palette`))
  (bind _returnvalue (`KismetArrayLibrary.Array_Length` _palette))
  (bind _returnvalue_2 (`KismetMathLibrary.Sqrt` (`KismetMathLibrary.Conv_IntToDouble` _returnvalue)))
  (bind _returnvalue_3 (`KismetMathLibrary.FCeil` _returnvalue_2))
  (bind _returnvalue_4 (`KismetMathLibrary.FFloor` _returnvalue_2))
  (`TextureBakerOutputBlueprintLibrary.AddTexture2DOutput` OutputTargets (make `TextureBakerOutputInfo` (select `bool` (`self.Square`) :`false` (make `IntPoint` (/ (+ _returnvalue -1 _returnvalue_4) _returnvalue_4) _returnvalue_4) :`true` (make `IntPoint` _returnvalue_3 _returnvalue_3)) "None" (`|GetArrayItem` _palette) "TMGS_NoMipmaps" "TSF_BGRA8" "Saturate" "TF_Nearest" "TA_Clamp" "TA_Clamp" (`self.sRGB`) (`self.Compression`) (`self.WithoutAlpha`)) (`KismetStringLibrary.JoinStringArray` (`|MakeArray` DirectoryPath (`self.TextureName`)) "/") (`|CreateDelegate` :!event `BakePalette`))
  (return))