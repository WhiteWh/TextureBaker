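; Texture baker Blueprint that bakes a tinted copy of a source Texture into an output asset of the same name in the given directory.
; RegisterOutputTarget matches the source's size and power-of-two padding, with configurable sRGB and compression settings.
; BakeTextureCopy prepares the source at imported resolution, uncompressed and without mipmaps, then draws it across the canvas with TintColor and alpha compositing.
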(fn `BakeTextureCopy`
  (params (Info :type "TextureBakerOutputInfo Structure") (bIsPreviewRender :type Boolean) (Canvas :type "Canvas Object Reference"))
  (returns (ReturnValue :type Boolean))
  (bind _returnvalue (`self.PrepareTexture` (`self.Texture`) (make `TextureBakerResourceRequirements` true true "TMGS_NoMipmaps")))
  (`Canvas.K2_DrawTexture` Canvas _returnvalue (0.0 0.0) (`KismetMathLibrary.Conv_IntPointToVector2D` Info_OutputDimensions) (0.0 0.0) (1.0 1.0) (`self.TintColor`) "BLEND_AlphaComposite" 0.0 (0.5 0.5))
  (return true))

(fn `InitialSettingsIsValid`
  (returns (ReturnValue :type Boolean))
  (return (`KismetSystemLibrary.IsValid` (`self.Texture`))))

(fn `RegisterOutputTarget`
  (params (DirectoryPath :type String))
  (returns (OutputTargets :type "Array of TextureBakerOutputWriteout Structure"))
  (bind _texture (`self.Texture`))
  (return (`|MakeArray` (`TextureBakerOutputBlueprintLibrary.MakeOutputWriteout` (`KismetStringLibrary.JoinStringArray` (`|MakeArray` DirectoryPath (`KismetSystemLibrary.GetObjectName` _texture)) "/") (make `TextureBakerOutputInfo` (make `IntPoint` (`Texture2D.Blueprint_GetSizeX` _texture) (`Texture2D.Blueprint_GetSizeY` _texture)) (`Texture.PowerOfTwoMode` _texture) (struct) "TMGS_FromTextureGroup" "TSF_BGRA8" "Saturate" (`self.UseSRGB`) (`self.CompressionSettings`) (`self.CompressWithoutAlpha`)) (`|CreateDelegate` :!event `BakeTextureCopy`)))))