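; Texture baker asset that bakes a color curve into a palette texture, one pixel per sample.
; It validates the name, curve and sample count, then registers a square or near-square output sized to fit the samples, with nearest filtering, clamping and no mipmaps.
; BakePalette samples the curve at even steps from its start time, stopping one step short of the end, and draws pixel boxes row by row.
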(fn `BakePalette`
  (params (Info :type "TextureBakerOutputInfo Structure") (bIsPreviewRender :type Boolean) (Canvas :type "Canvas Object Reference"))
  (returns (ReturnValue :type Boolean))
  (bind _curve (`self.Curve`))
  (bind (_mintime _maxtime) (`CurveBase.GetTimeRange` _curve))
  (for _index (range (`self.Samples`))
    (`Canvas.K2_DrawBox` (`local.Canvas`) (+ (`KismetMathLibrary.MakeVector2D` (`KismetMathLibrary.Conv_IntToDouble` (mod _index (break `IntPoint` (break `TextureBakerOutputInfo` Info)))) (`KismetMathLibrary.Conv_IntToDouble` (/ _index (break `IntPoint` (break `TextureBakerOutputInfo` Info))))) 0.5) (0.5 0.5) 1.0 (`CurveLinearColor.GetLinearColorValue` _curve (+ _mintime (* _index (/ (- _maxtime _mintime) (`KismetMathLibrary.Conv_IntToDouble` (`self.Samples`))))))))
  (return true))

(fn `InitialSettingsIsValid`
  (returns (ReturnValue :type Boolean))
  (return (and (not (`KismetStringLibrary.IsEmpty` (`self.TextureName`))) (`KismetSystemLibrary.IsValid` (`self.Curve`)) (> (`self.Samples`) 0))))

(fn `RegisterOutputTarget`
  (params (DirectoryPath :type String) (OutputTargets :type "TextureBakerOutputList Structure (by ref)"))
  (bind _samples (`self.Samples`))
  (bind _curve (`self.Curve`))
  (bind _returnvalue (`KismetMathLibrary.Sqrt` (`KismetMathLibrary.Conv_IntToDouble` _samples)))
  (bind _returnvalue_2 (`KismetMathLibrary.FCeil` _returnvalue))
  (bind _returnvalue_3 (`KismetMathLibrary.FFloor` _returnvalue))
  (`TextureBakerOutputBlueprintLibrary.AddTexture2DOutput` OutputTargets (make `TextureBakerOutputInfo` (select `bool` (`self.Square`) :`false` (make `IntPoint` (/ (+ _samples -1 _returnvalue_3) _returnvalue_3) _returnvalue_3) :`true` (make `IntPoint` _returnvalue_2 _returnvalue_2)) "None" (`CurveLinearColor.GetLinearColorValue` _curve (`CurveBase.GetTimeRange` _curve)) "TMGS_NoMipmaps" "TSF_BGRA8" "Saturate" "TF_Nearest" "TA_Clamp" "TA_Clamp" (`self.sRGB`) (`self.Compression`) (`self.WithoutAlpha`)) (`KismetStringLibrary.JoinStringArray` (`|MakeArray` DirectoryPath (`self.TextureName`)) "/") (`|CreateDelegate` :!event `BakePalette`))
  (return))