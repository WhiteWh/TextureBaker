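; BakeCurve_BP is a texture baker that renders a linear color curve asset into a horizontal gradient texture.
; It validates the curve and dimensions, then registers an output named after the curve with configurable padding, mip, normalization, sRGB and compression settings.
; The bake draws one vertical line per pixel column on a Canvas, sampling the curve across its time range from left to right.
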(fn `BakeLinearGradient`
  (params (Info :type "TextureBakerOutputInfo Structure") (bIsPreviewRender :type Boolean) (Canvas :type "Canvas Object Reference"))
  (returns (ReturnValue :type Boolean))
  (bind (_x _y) (break `IntPoint` Info_OutputDimensions))
  (bind (_mintime _maxtime) (`CurveBase.GetTimeRange` (`self.GradientCurve`)))
  (for _index (range _x)
    (bind _returnvalue (`KismetMathLibrary.Conv_IntToDouble` _index))
    (bind _returnvalue_2 (+ (`KismetMathLibrary.MakeVector2D` _returnvalue (`KismetMathLibrary.Conv_IntToDouble` _y)) (0.5 0.0)))
    (`Canvas.K2_DrawLine` (`local.Canvas`) (* _returnvalue_2 (1.0 0.0)) (* _returnvalue_2 (1.0 1.0)) 1.0 (`CurveLinearColor.GetLinearColorValue` (`self.GradientCurve`) (`KismetMathLibrary.Lerp` _mintime _maxtime (/ _returnvalue (`KismetMathLibrary.Conv_IntToDouble` _x))))))
  (return true))

(fn `InitialSettingsIsValid`
  (returns (ReturnValue :type Boolean))
  (bind (_texturedimensions_x _texturedimensions_y) (break `IntPoint` (`self.TextureDimensions`)))
  (return (and (`KismetSystemLibrary.IsValid` (`self.GradientCurve`)) (> (`KismetMathLibrary.Min` _texturedimensions_x _texturedimensions_y) 0))))

(fn `RegisterOutputTarget`
  (params (DirectoryPath :type String))
  (returns (OutputTargets :type "Array of TextureBakerOutputWriteout Structure"))
  (bind _gradientcurve (`self.GradientCurve`))
  (return (`|MakeArray` (`TextureBakerOutputBlueprintLibrary.MakeOutputWriteout` (`KismetStringLibrary.JoinStringArray` (`|MakeArray` DirectoryPath (`KismetSystemLibrary.GetObjectName` _gradientcurve)) "/") (make `TextureBakerOutputInfo` (`self.TextureDimensions`) (`self.PaddingMode`) (`CurveLinearColor.GetLinearColorValue` _gradientcurve 0.0) (`self.MipGenSettings`) "TSF_BGRA8" (`self.Normalization`) (`self.sRGB`) (`self.Compression`) (`self.WithoutAlpha`)) (`|CreateDelegate` :!event `BakeLinearGradient`)))))